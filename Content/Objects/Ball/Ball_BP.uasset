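; Physics ball actor that enables simulation on Release and drives rolling and impact sounds.
; Each tick, a short downward trace detects ground; while on it, the rolling sound stops at zero velocity and, when moving, Play is called only if already playing.
; Hits above an impulse threshold play an impact cue at the contact point, with volume scaled by excess impulse, which is also printed.
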(event `self.ReceiveTick`
  (params (DeltaSeconds :type "Float (single-precision)"))
  (bind _returnvalue (`self.K2_GetActorLocation`))
  (bind _rollingsound (`self.RollingSound`))
  (bind (_outhit _returnvalue_2) (`KismetSystemLibrary.LineTraceSingle` _returnvalue (- _returnvalue (0.0 0.0 25.0)) "TraceTypeQuery1"))
  (if _returnvalue_2
    (bind _returnvalue_3 (`PrimitiveComponent.GetPhysicsLinearVelocity` (`self.StaticMesh`) "None"))
    (if (> (`KismetMathLibrary.VSize` _returnvalue_3) 0.0)
      (if (`AudioComponent.IsPlaying` _rollingsound)
        (`AudioComponent.Play` _rollingsound 0.0))
      (else
        (`AudioComponent.Stop` _rollingsound)))))

(event `Release`
  (`PrimitiveComponent.SetSimulatePhysics` (`self.StaticMesh`) true))

(event `self.ReceiveHit`
  (params (MyComp :type "PrimitiveComponent Object Reference") (Other :type "Actor Object Reference") (OtherComp :type "PrimitiveComponent Object Reference") (bSelfMoved :type Boolean) (HitLocation :type "Vector Structure") (HitNormal :type "Vector Structure") (NormalImpulse :type "Vector Structure") (Hit :type "HitResult Structure (by ref)"))
  (bind _returnvalue (`KismetMathLibrary.VSize` NormalImpulse))
  (bind _returnvalue_2 (/ (- _returnvalue 6000.0) 20000.0))
  (if (> _returnvalue 6000.0)
    (`KismetSystemLibrary.PrintString` (`KismetStringLibrary.Conv_DoubleToString` _returnvalue_2))
    (`GameplayStatics.PlaySoundAtLocation` "/Game/Objects/Ball/BallHit-1_Cue.BallHit-1_Cue" HitLocation (struct) _returnvalue_2 1.0 0.0 null null null null)))

(fn `UserConstructionScript`)